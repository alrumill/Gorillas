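; Character Blueprint for a second gorilla variant, apparently boss-derived, that handles rock-throw visuals and a one-time tame announcement.
; Anim notifies TakeRock and ThrowRock show and hide the RockMesh.
; Server Tick treats a TargetingTeam in the player range as tamed, latches WasTamed and broadcasts a billboard notification with empty text and boss-head icon.
; Possession resets player pawn 0's scale to one, and the attack-weight override returns zero.
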(event EventPossessed
  (params (NewController :type Controller%20Object%20Reference))
  (Transformation|SetActorScale3D (Game|Player|GetPlayerPawn 0) (Math|Vector|MakeVector 1.0 1.0 1.0)))

(event EventBlueprintAnimNotifyCustomEvent
  (params (CustomEventName :type Name :default "None") (MeshComp :type Skeletal%20Mesh%20Component%20Object%20Reference) (Animation :type Anim%20Sequence%20Base%20Object%20Reference) (AnimNotifyObject :type Anim%20Notify%20Object%20Reference))
  (bind _rockmesh (Variables|Default|GetRockMesh))
  (if (Utilities|Name|Equal(Name) CustomEventName "TakeRock")
    (Development|SetHiddeninGame _rockmesh false false)
    (elif (Utilities|Name|Equal(Name) CustomEventName "ThrowRock")
      (Development|SetHiddeninGame _rockmesh true false))))

(event EventTick
  (params (DeltaSeconds :type Float%20%28single-precision%29))
  (|CallParentFunction DeltaSeconds)
  (if (Math|Boolean|ANDBoolean (Networking|IsServer) (not (Variables|Default|GetbWasTamed)) (>= (Variables|Default|GetTargetingTeam) 50000))
    (Variables|Default|SetbWasTamed true)
    (bind _asshootergamemode (Utilities|Casting|CastToShooterGameMode (Game|GetGameMode)))
    (Class|ShooterGameMode|SendServerNotification _asshootergamemode (Utilities|String|Append (Utilities|String|Append "" "") "") "(R=1.000000,G=0.054220,B=0.579979,A=1.000000)" 2.0 6.75 "/Game/PrimalEarth/UI/Empty_GorillaBossHead_Icon.Empty_GorillaBossHead_Icon" 0 -1 -1 true)))

(fn ConstructionScript
  (|CallParentFunction))

(fn BlueprintGetAttackWeight
  (params (AttackIndex :type Integer) (inputWeight :type Float%20%28single-precision%29) (distance :type Float%20%28single-precision%29) (attackRangeOffset :type Float%20%28single-precision%29) (OtherTarget :type Actor%20Object%20Reference))
  (return 0.0))

(fn BPCharacterSleeped)

(fn BPUnstasis)